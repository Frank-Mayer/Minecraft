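; BPC_Priest is an NPC character that faces its movement direction, walks home and offers the player a branching service dialogue.
; While nearly stationary, Tick uses gates to cache the BP_PriestHouse location, issue the move home and show the dialogue when the player is close.
; MoveHome opens the movement gate, then the dialogue gate after a delay.
; BeginPlay and Interact face the player, and the construction script tints the skin material.
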(event `self.ReceiveTick`
  (params (DeltaSeconds :type "Float (single-precision)"))
  (bind _returnvalue (`self.GetVelocity`))
  (bind (_returnvalue_2 _createdcorrectly) (`/Game/GUI/BPL_UI.CreateDialogueBranch` "..." "PriestTxt02" "What kind of service?" "" "" "" (`/Game/GUI/BPL_UI.CreateDialogueBranch` "David" "PriestTxt03" "I agree" "" "" "" null null null null "/Engine/VREditor/Sounds/VR_click1_Cue.VR_click1_Cue") null null null "/Engine/VREditor/Sounds/VR_click1_Cue.VR_click1_Cue"))
  (if (> (`KismetMathLibrary.VSizeXY` _returnvalue) 10.0)
    (`SceneComponent.K2_SetWorldRotation` (`self.Mesh`) (`KismetMathLibrary.MakeRotator` (.roll (`KismetMathLibrary.FindLookAtRotation` (`KismetMathLibrary.MakeVector` 0.0) _returnvalue)) (.pitch (`KismetMathLibrary.FindLookAtRotation` (`KismetMathLibrary.MakeVector` 0.0) _returnvalue)) (- (.yaw (`KismetMathLibrary.FindLookAtRotation` (`KismetMathLibrary.MakeVector` 0.0) _returnvalue)) 90.0)) false false)
    (else
      (`|ExecutionSequence`
        (:`then_0`
          (`/Engine/EditorBlueprintResources/StandardMacros.Gate` false :!label _label
            (:`Exit`
              (bind _outactors (`GameplayStatics.GetAllActorsOfClass` "/Game/WorldGenerator/City/BP_PriestHouse.BP_PriestHouse_C"))
              (if (> (`KismetArrayLibrary.Array_Length` _outactors) 0)
                (set `self.HomeLocation` (`SceneComponent.K2_GetComponentLocation` (`/Game/WorldGenerator/City/BP_PriestHouse.Billboard` (`|GetArrayItem` _outactors))))
                (goto _label :!via `Close`)))))
        (:`then_1`
          (`/Engine/EditorBlueprintResources/StandardMacros.Gate` true :!label _label_2
            (:`Exit`
              (if (< (`self.GetDistanceTo` self (`GameplayStatics.GetPlayerPawn` 0)) 200.0)
                (`|ExecutionSequence`
                  (:`then_0`
                    (goto _label_2 :!via `Close`))
                  (:`then_1`
                    (if _createdcorrectly
                      (`UserWidget.AddToViewport` _returnvalue_2 0)))
                  (:`then_2`
                    (goto _label_3 :!via `Close`)))))))
        (:`then_2`
          (`/Engine/EditorBlueprintResources/StandardMacros.Gate` true :!label _label_3
            (:`Exit`
              (`AIBlueprintHelperLibrary.SimpleMoveToLocation` (`self.GetController`) (`self.HomeLocation`)))))))))

(event `self.ReceiveBeginPlay`
  (`SceneComponent.K2_SetWorldRotation` (`self.Mesh`) (`KismetMathLibrary.MakeRotator` 0.0 0.0 (- (.yaw (`KismetMathLibrary.FindLookAtRotation` (`self.K2_GetActorLocation` self) (`self.K2_GetActorLocation` (`GameplayStatics.GetPlayerPawn` 0)))) 90.0)) false false :!label _label_4))

(event `MoveHome`
  (`|ExecutionSequence`
    (:`then_0`
      (goto _label_3 :!via `Open`))
    (:`then_1`
      (`KismetSystemLibrary.Delay` 3.0)
      (goto _label_2 :!via `Open`))))

(event `/Game/WorldGenerator/Interactables/BPI_Interaction.interact`
  (params (OwningPlayer :type "PlayerController Object Reference"))
  (goto _label_4))

(event `/Game/GUI/BPI_Dialogue.Trigger`
  (params (FunctionName :type String))
  (`KismetSystemLibrary.K2_SetTimer` self FunctionName 0.1 false 0.1))

(fn `UserConstructionScript`
  (bind _returnvalue (`KismetMaterialLibrary.CreateDynamicMaterialInstance` (`self.Skin`) (`KismetStringLibrary.Conv_StringToName` (`KismetStringLibrary.Concat_StrStr` (`KismetSystemLibrary.GetDisplayName` self) "_Skin"))))
  (set `self.CustomSkinMaterial` _returnvalue)
  (`MaterialInstanceDynamic.SetVectorParameterValue` (`self.CustomSkinMaterial`) "Color" (`self.ClothingColor`))
  (`PrimitiveComponent.SetMaterial` (`self.Mesh`) 0 (`self.CustomSkinMaterial`)))