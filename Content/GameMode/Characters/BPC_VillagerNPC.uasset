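; Villager NPC character Blueprint that gives each villager its own clothing color and turns its body to face where it moves.
; The construction script creates a dynamic skin material and applies ClothingColor, or a dark random color when that color is black.
; SetCustomColor overrides the color at runtime.
; On Tick, while horizontal speed exceeds a small threshold, the mesh rotates to the velocity direction with a 90-degree yaw offset.
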(event `self.ReceiveTick`
  (params (DeltaSeconds :type "Float (single-precision)"))
  (bind _returnvalue (`self.GetVelocity`))
  (if (> (`KismetMathLibrary.VSizeXY` _returnvalue) 10.0)
    (`SceneComponent.K2_SetWorldRotation` (`self.Mesh`) (`KismetMathLibrary.MakeRotator` (.roll (`KismetMathLibrary.FindLookAtRotation` (`KismetMathLibrary.MakeVector` 0.0) _returnvalue)) (.pitch (`KismetMathLibrary.FindLookAtRotation` (`KismetMathLibrary.MakeVector` 0.0) _returnvalue)) (- (.yaw (`KismetMathLibrary.FindLookAtRotation` (`KismetMathLibrary.MakeVector` 0.0) _returnvalue)) 90.0)) false false)))

(fn `RandomColor`
  (returns (LinearColor :type "LinearColor Structure"))
  (return (make `LinearColor` (`KismetMathLibrary.RandomFloatInRange` 0.05 0.125) (`KismetMathLibrary.RandomFloatInRange` 0.05 0.125) (`KismetMathLibrary.RandomFloatInRange` 0.05 0.125) 1.0)))

(fn `Set Custom Color`
  (params (Value :type "LinearColor Structure" :default (struct :`R` 0.219526 :`G` 0.052861 :`B` 0.114435 :`A` 1.0)))
  (bind (_r _g _b) (break `LinearColor` Value))
  (set `self.ClothingColor` (make `LinearColor` _r _g _b 1.0))
  (`MaterialInstanceDynamic.SetVectorParameterValue` (`self.CustomSkinMaterial`) "Color" (`self.ClothingColor`))
  (`PrimitiveComponent.SetMaterial` (`self.Mesh`) 0 (`self.CustomSkinMaterial`))
  (return))

(fn `UserConstructionScript`
  (bind (_r _g _b) (break `LinearColor` (`self.ClothingColor`)))
  (bind _returnvalue (`KismetMaterialLibrary.CreateDynamicMaterialInstance` (`self.Skin`) (`KismetStringLibrary.Conv_StringToName` (`KismetStringLibrary.Concat_StrStr` (`KismetSystemLibrary.GetDisplayName` self) "_Skin"))))
  (set `self.CustomSkinMaterial` _returnvalue)
  (`MaterialInstanceDynamic.SetVectorParameterValue` (`self.CustomSkinMaterial`) "Color" (`KismetMathLibrary.SelectColor` (`KismetMathLibrary.MakeColor` _r _g _b) (`self.RandomColor`) (or (!= _r 0.0) (!= _g 0.0) (!= _b 0.0))))
  (`PrimitiveComponent.SetMaterial` (`self.Mesh`) 0 (`self.CustomSkinMaterial`)))