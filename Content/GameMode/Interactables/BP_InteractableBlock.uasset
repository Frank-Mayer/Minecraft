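; BP_InteractableBlock is an interactable block actor that opens a UI widget for the player who interacts with it.
; Its Construct function stores a Material and Widget class and applies the material to the Block component.
; The construction script also applies the material and sets a large uniform actor scale.
; Interact adds the widget to that player's screen, switches to UI-only input with mouse lock and shows the cursor.
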(event `/Game/WorldGenerator/Interactables/BPI_Interaction.interact`
  (params (OwningPlayer :type "PlayerController Object Reference"))
  (bind _returnvalue (`|CreateWidget` (`self.Widget`) OwningPlayer))
  (`UserWidget.AddToPlayerScreen` _returnvalue 0)
  (`WidgetBlueprintLibrary.SetInputMode_UIOnlyEx` OwningPlayer _returnvalue "LockAlways")
  (set `PlayerController.bShowMouseCursor` true OwningPlayer))

(fn `Construct`
  (params (Material :type "MaterialInterface Object Reference") (Widget :type "UserWidget Class Reference"))
  (bind _output_get (set `self.Material` Material))
  (set `self.Widget` Widget)
  (`PrimitiveComponent.SetMaterial` (`self.Block`) 0 _output_get))

(fn `UserConstructionScript`
  (`PrimitiveComponent.SetMaterial` (`self.Block`) 0 (`self.Material`))
  (`self.SetActorScale3D` self (100.0 100.0 100.0)))