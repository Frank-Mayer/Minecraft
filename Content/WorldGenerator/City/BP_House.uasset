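; BP_House is a city building for the world generator that culls itself by distance and reacts when the player character (Steve) goes inside.
; A looping timer hides it beyond the WorldGeneratorMaster's view distance in chunks.
; The construction script finds the window material slot.
; Box overlaps swap that slot to M_Window2S inside and back outside, while toggling Steve's auto-jump and Interior flag.
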(event `self.ReceiveBeginPlay`
  (`KismetSystemLibrary.K2_SetTimer` null "ChekDistance" 1.0 true))

(event `ChekDistance`
  (bind _outactors (`GameplayStatics.GetAllActorsOfClass` "/Game/WorldGenerator/WorldGeneratorMaster.WorldGeneratorMaster_C"))
  (bind _output (`|GetArrayItem` _outactors))
  (`self.SetActorHiddenInGame` (> (`self.GetDistanceTo` self (`GameplayStatics.GetPlayerPawn` 0)) (`KismetMathLibrary.Conv_IntToDouble` (* (`/Game/WorldGenerator/WorldGeneratorMaster.ViewDistance` _output) (`/Game/WorldGenerator/WorldGeneratorMaster.ChunkSize` _output))))))

(event `self.Box.OnComponentBeginOverlap`
  (params (OverlappedComponent :type "PrimitiveComponent Object Reference") (OtherActor :type "Actor Object Reference") (OtherComp :type "PrimitiveComponent Object Reference") (OtherBodyIndex :type Integer) (bFromSweep :type Boolean) (SweepResult :type "HitResult Structure (by ref)"))
  (`self.Enter` OtherActor))

(event `self.Box.OnComponentEndOverlap`
  (params (OverlappedComponent :type "PrimitiveComponent Object Reference") (OtherActor :type "Actor Object Reference") (OtherComp :type "PrimitiveComponent Object Reference") (OtherBodyIndex :type Integer))
  (`self.Leave` OtherActor))

(fn `Enter`
  (params (Object :type "Object Object Reference"))
  (bind _assteve (cast `/Game/GameMode/Steve` Object)
    (:`then`
      (if (`self.SetMaterial`)
        (`PrimitiveComponent.SetMaterial` (`self.StaticMesh`) (`self.GlassMaterialIndex`) "/Game/WorldGenerator/TerrainMaterials/M_Window2S.M_Window2S"))
      (set `/Game/GameMode/Steve.UseAutoJump` false _assteve)
      (set `/Game/GameMode/Steve.interior` true _assteve))
    (:`CastFailed`
      _))
  (return))

(fn `Leave`
  (params (Object :type "Object Object Reference"))
  (bind _assteve (cast `/Game/GameMode/Steve` Object))
  (if (`self.SetMaterial`)
    (`PrimitiveComponent.SetMaterial` (`self.StaticMesh`) (`self.GlassMaterialIndex`) "/Game/WorldGenerator/TerrainMaterials/M_Window.M_Window"))
  (set `/Game/GameMode/Steve.UseAutoJump` true _assteve)
  (set `/Game/GameMode/Steve.interior` false _assteve))

(fn `UserConstructionScript`
  (for (_array_element _array_index) (`MeshComponent.GetMaterials` (`self.StaticMesh`))
    (if (== _array_element "/Game/WorldGenerator/TerrainMaterials/M_Window.M_Window")
      (set `self.GlassMaterialIndex` _array_index)
      (set `self.SetMaterial` true)
      (break))))