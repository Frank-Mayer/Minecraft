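; BP_Door is a door actor for the city world generator that opens when something overlaps its trigger box and closes when the overlap ends.
; Unless Locked, overlap events set DoorOpen, snap the Arrow component's relative rotation between open and closed angles, and play 2D open and close sounds.
; The construction script shows the lock state by giving the Cube an iron material when locked and oak when unlocked.
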(event `self.Box.OnComponentBeginOverlap`
  (params (OverlappedComponent :type "PrimitiveComponent Object Reference") (OtherActor :type "Actor Object Reference") (OtherComp :type "PrimitiveComponent Object Reference") (OtherBodyIndex :type Integer) (bFromSweep :type Boolean) (SweepResult :type "HitResult Structure (by ref)"))
  (if (not (`self.Locked`))
    (set `self.DoorOpen` true)
    (`SceneComponent.K2_SetRelativeRotation` (`self.Arrow`) (struct :`Pitch` 90.0 :`Yaw` 90.0) false false)
    (`GameplayStatics.PlaySound2D` "/Game/Sounds/Door/DoorOpen.DoorOpen" 1.0 1.0 0.0 null null)))

(event `self.Box.OnComponentEndOverlap`
  (params (OverlappedComponent :type "PrimitiveComponent Object Reference") (OtherActor :type "Actor Object Reference") (OtherComp :type "PrimitiveComponent Object Reference") (OtherBodyIndex :type Integer))
  (if (not (`self.Locked`))
    (set `self.DoorOpen` false)
    (`SceneComponent.K2_SetRelativeRotation` (`self.Arrow`) (struct :`Pitch` 90.0) false false)
    (`GameplayStatics.PlaySound2D` "/Game/Sounds/Door/DoorClose.DoorClose" 1.0 1.0 0.0 null null)))

(fn `UserConstructionScript`
  (`PrimitiveComponent.SetMaterial` (`self.Cube`) 0 (select `bool` (`self.Locked`) :`false` "/Game/WorldGenerator/TerrainMaterials/M_OakDoor.M_OakDoor" :`true` "/Game/WorldGenerator/TerrainMaterials/MInst_IronDoor.MInst_IronDoor" :!type "MaterialInterface Object Reference")))